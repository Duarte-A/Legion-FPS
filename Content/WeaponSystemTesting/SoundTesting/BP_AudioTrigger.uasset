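; BP_AudioTrigger is a box trigger volume that starts a 2D soundtrack when the player character overlaps it.
; An optional flag first stops the stored sound on every BP_AudioTrigger in the level, so one track replaces the others.
; Each trigger keeps the spawned audio component for later stopping, and every overlap spawns a new one without checking whether one is already playing.
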(event `self.Box.OnComponentBeginOverlap`
  (params (OverlappedComponent :type "PrimitiveComponent Object Reference") (OtherActor :type "Actor Object Reference") (OtherComp :type "PrimitiveComponent Object Reference") (OtherBodyIndex :type Integer) (bFromSweep :type Boolean) (SweepResult :type "HitResult Structure (by ref)"))
  (if (== OtherActor (`GameplayStatics.GetPlayerCharacter` 0))
    (if (`self.TurnOffAllOtherSounds`)
      (bind _outactors (`GameplayStatics.GetAllActorsOfClass` "BP_AudioTrigger_C"))
      (for _array_element _outactors
        (bind _sound2d (`/Game/WeaponSystemTesting/SoundTesting/BP_AudioTrigger.Sound2D` _array_element))
        (`/Engine/EditorBlueprintResources/StandardMacros.IsValid` _sound2d
          (:`Is Valid`
            (`AudioComponent.Stop` _sound2d)))))
    (bind _returnvalue (`GameplayStatics.SpawnSound2D` (`self.SoundTrackToPlay`) 1.0 1.0 0.0 null))
    (set `self.Sound2D` _returnvalue)))

(fn `UserConstructionScript`)