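; Shotgun weapon Blueprint that replaces its parent's FireLineTrace with a multi-pellet hitscan shot, without calling the parent version.
; Each pellet traces from the player 0 camera in a random direction within the spread cone, passing per-bullet damage info to BPCAttacks.
; The shot then plays one firing sound, attaches a muzzle flash at the barrel socket and removes one round from the magazine.
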(fn `FireLineTrace`
  (bind _barrelsocketname (`self.BarrelSocketName`))
  (bind _itemmodel (`self.ItemModel`))
  (bind _transformcomponent (`PlayerCameraManager.TransformComponent` (`GameplayStatics.GetPlayerCameraManager` 0)))
  (bind _returnvalue (`SceneComponent.K2_GetComponentLocation` _transformcomponent))
  (for _ (range 1 (+ (`self.NumberOfPallets`) 1))
    (`/Game/P01_Content/AI/BP/V2-SmartAI/RAIS-Template/TP-Player/Attacks/BPC-Attacks.LineTraceFire` (`self.BPC-Attacks`) _returnvalue (+ _returnvalue (* (`KismetMathLibrary.RandomUnitVectorInConeInDegrees` (`SceneComponent.GetForwardVector` _transformcomponent) (`self.SpreadAngle`)) (`self.LineTraceRange`))) (make `/Game/P01_Content/AI/BP/V2-SmartAI/NDS-NewDamageSystem/Damage-Logic/S_DamageInfo` (`self.DamagePerBullet`) "NewEnumerator2" "NewEnumerator1")))
  (`GameplayStatics.PlaySoundAtLocation` (`self.WeaponFiringSound`) (`SceneComponent.K2_GetComponentLocation` (`self.ItemModel`)) (struct) (`self.WeaponFireSoundMultiplier`) 1.0 0.0 null null null null)
  (`GameplayStatics.SpawnEmitterAttached` (`self.MuzzleFlash`) _itemmodel _barrelsocketname (`SceneComponent.GetSocketLocation` _itemmodel _barrelsocketname) (struct) (1.0 1.0 1.0) "KeepWorldPosition")
  (set `self.CurrentAmmoInMag` (- (`self.CurrentAmmoInMag`) 1)))

(fn `UserConstructionScript`
  (`parent.UserConstructionScript`))