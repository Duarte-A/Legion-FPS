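; BP_LocationObjective is a travel objective that the player starts and completes by overlapping two trigger components, StartPoint and EndPoint.
; The first player overlap at StartPoint sets ObjectiveInProgress, caches BP_FirstPersonGameMode and calls StartObjective with ObjectiveTextID.
; EndPoint then calls ObjectiveComplete, but never clears the flag, so later overlaps report completion again.
; Both steps play a feedback sound at world origin rather than at the trigger.
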(event `self.StartPoint.OnComponentBeginOverlap`
  (params (OverlappedComponent :type "PrimitiveComponent Object Reference") (OtherActor :type "Actor Object Reference") (OtherComp :type "PrimitiveComponent Object Reference") (OtherBodyIndex :type Integer) (bFromSweep :type Boolean) (SweepResult :type "HitResult Structure (by ref)"))
  ;[1 1 1] Start Location Objective
  (if (== OtherActor (`GameplayStatics.GetPlayerCharacter` 0))
    (if (not (`self.ObjectiveInProgress`))
      (set `self.ObjectiveInProgress` true)
      (bind _asbp_first_person_game_mode (cast `/Game/FirstPerson/Blueprints/BP_FirstPersonGameMode` (`GameplayStatics.GetGameMode`)))
      (`/Game/FirstPerson/Blueprints/BP_FirstPersonGameMode.StartObjective` _asbp_first_person_game_mode (`self.ObjectiveText/ID`))
      (`GameplayStatics.PlaySoundAtLocation` "/Engine/VREditor/Sounds/UI/Click_on_Button_Cue.Click_on_Button_Cue" (0.0 0.0 0.0) (struct) 1.0 1.0 0.0 null null null null))))

(event `self.EndPoint.OnComponentBeginOverlap`
  (params (OverlappedComponent :type "PrimitiveComponent Object Reference") (OtherActor :type "Actor Object Reference") (OtherComp :type "PrimitiveComponent Object Reference") (OtherBodyIndex :type Integer) (bFromSweep :type Boolean) (SweepResult :type "HitResult Structure (by ref)"))
  ;[1 1 1] End Location Objective
  (if (== OtherActor (`GameplayStatics.GetPlayerCharacter` 0))
    (if (`self.ObjectiveInProgress`)
      (`/Game/FirstPerson/Blueprints/BP_FirstPersonGameMode.ObjectiveComplete` (stale `self.StartPoint.OnComponentBeginOverlap` _asbp_first_person_game_mode) (`self.ObjectiveText/ID`))
      (`GameplayStatics.PlaySoundAtLocation` "/Engine/VREditor/Sounds/UI/Camera_Shutter.Camera_Shutter" (0.0 0.0 0.0) (struct) 1.0 1.0 0.0 null null null null))))

(fn `UserConstructionScript`)