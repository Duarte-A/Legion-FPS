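; Enemy spawner actor that holds a queue of enemy classes and spawns them at its own transform.
; Queued enemies spawn immediately if no enemy overlaps its sphere; once StartSpawning runs, a looping timer also spawns the next entry, without that check.
; Each spawn binds to the enemy's death event, and EnemyDefeated forwards defeats to BP_FirstPersonGameMode.
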(event `StartSpawning`
  (`KismetSystemLibrary.K2_SetTimerDelegate` (delegate `TryToSpawn`) 2.0 true))

(event `TryToSpawn`
  (`self.SpawnEnemy`))

(event `EnemyDefeated`
  (bind _asbp_first_person_game_mode (cast `/Game/FirstPerson/Blueprints/BP_FirstPersonGameMode` (`GameplayStatics.GetGameMode`)))
  (`/Game/FirstPerson/Blueprints/BP_FirstPersonGameMode.OnEnemyDefeated` _asbp_first_person_game_mode))

(fn `AddEnemyToQueue`
  (params (EnemyClass :type "/Game/P01_Content/AI/BP/V2-SmartAI/RAIS-Template/AI-Characters/BP-Enemy-Base Class Reference (by ref)"))
  (`KismetArrayLibrary.Array_Add` (`self.EnemyQueue`) EnemyClass)
  (if (not (`KismetArrayLibrary.Array_IsValidIndex` (`PrimitiveComponent.GetOverlappingActors` (`self.Sphere`) "/Game/P01_Content/AI/BP/V2-SmartAI/RAIS-Template/AI-Characters/BP-Enemy-Base.BP-Enemy-Base_C")))
    (`self.SpawnEnemy`)))

(fn `SpawnEnemy`
  (returns (Success :type Boolean))
  (if (`KismetArrayLibrary.Array_IsValidIndex` (`self.EnemyQueue`))
    (bind _returnvalue (`|SpawnActorFromClass` (`|GetArrayItem` (`self.EnemyQueue`)) (`self.GetTransform`) "AdjustIfPossibleButAlwaysSpawn" "MultiplyWithRoot" null 2 2.0 null))
    (add `/Game/P01_Content/AI/BP/V2-SmartAI/RAIS-Template/AI-Characters/BP-Enemy-Base.OnDeath` _returnvalue (`|CreateDelegate` :!event `EnemyDefeated`))
    (`KismetArrayLibrary.Array_Remove` (`self.EnemyQueue`))
    (return true)
    (else
      (return false))))

(fn `UserConstructionScript`)