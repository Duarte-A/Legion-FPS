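; BP_DmgAmt is a short-lived actor that displays a damage amount as a moving popup.
; On BeginPlay it passes its DmgAmt value to the WBP_DmgAmt widget in its widget component.
; The TL_Move timeline then lerps the actor from its spawn location to a fixed raised, diagonal world-space offset and destroys it when finished.
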(event `self.ReceiveBeginPlay`
  (bind _aswbp_dmg_amt (cast `/Game/WeaponSystemTesting/Widgets/WBP_DmgAmt` (`WidgetComponent.GetWidget` (`self.Widget`))))
  (set `/Game/WeaponSystemTesting/Widgets/WBP_DmgAmt.DmgAmt` (`self.Dmg Amt`) _aswbp_dmg_amt)
  (bind _output_get (set `self.StartLocation` (`self.K2_GetActorLocation`)))
  (set `self.EndLocation` (+ _output_get (-25.0 -25.0 50.0)))
  (bind (_direction _move_track) (`Timeline|TL_Move`)
    (:`Update`
      (`self.K2_SetActorLocation` (`KismetMathLibrary.VLerp` (`self.StartLocation`) (`self.EndLocation`) _move_track)))
    (:`Finished`
      (`self.K2_DestroyActor`))))

(fn `UserConstructionScript`)