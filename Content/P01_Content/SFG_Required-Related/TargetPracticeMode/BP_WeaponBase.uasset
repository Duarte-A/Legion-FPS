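; Base weapon Blueprint for target practice mode, handling ammo, firing and timed reloads, with an empty WeaponTrace event as the hook for shot logic.
; FireWeaponTrace spends a round and calls WeaponTrace, reloading automatically on an empty magazine.
; Automatic and manual reloads share a DoOnce gate that shows a reload bar widget, waits ReloadTime, then refills ammo.
; Helper functions play muzzle flash and sound, and return the FOV multiplier.
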(event `WeaponTrace`)

(event `self.ReceiveBeginPlay`
  (set `self.Ammo` (`self.MaxMagazineAmmo`)))

(event `/Game/P01_Content/SFG_Required-Related/TargetPracticeMode/BPI_TraceWeapon.FireWeaponTrace`
  ;[0 0 0] Fire Weapon Logic
  (`/Game/P01_Content/SFG_Required-Related/TargetPracticeMode/BPML_Comparisons.INT<=INT` (`self.Ammo`)
    (:`True`
      (`self.ReloadWeapon`))
    (:`False`
      (set `self.Ammo` (- (`self.Ammo`) 1))
      (`self.WeaponTrace`)
      (`/Game/P01_Content/SFG_Required-Related/TargetPracticeMode/BPML_Comparisons.INT<=INT` (`self.Ammo`)
        (:`True`
          (`self.ReloadWeapon`))))))

(event `ReloadWeapon`
  ;[0 0 0] Reload Weapon
  (`/Engine/EditorBlueprintResources/StandardMacros.DoOnce` false :!label _label
    (:`Completed`
      (bind _returnvalue (`|CreateWidget` "/Game/P01_Content/SFG_Required-Related/TargetPracticeMode/WBP_ReloadBar.WBP_ReloadBar_C"))
      (`/Game/P01_Content/SFG_Required-Related/TargetPracticeMode/WBP_ReloadBar.ReloadAnimation` _returnvalue (`self.ReloadTime`))
      (`UserWidget.AddToViewport` _returnvalue 0)
      (`KismetSystemLibrary.Delay` (`self.ReloadTime`))
      (set `self.Ammo` (`self.MaxMagazineAmmo`))
      (goto _label :!via `Reset`))))

(event `/Game/P01_Content/SFG_Required-Related/TargetPracticeMode/BPI_TraceWeapon.Reload`
  ;[0 0 0] Reload Weapon
  (goto _label))

(fn `GetFOVMultiplier`
  (returns (FOVMultiplier :type "Float (double-precision)"))
  (return (`self.FOVMultiplier`)))

(fn `UserConstructionScript`)

(fn `WeaponFireEffects`
  (bind _returnvalue_location (`KismetMathLibrary.BreakTransform` (`SceneComponent.K2_GetComponentToWorld` (`self.Arrow`))))
  (`ActorComponent.Activate` (`self.P_AssaultRifle_MuzzleFlash`) false)
  (`GameplayStatics.SpawnSoundAtLocation` (`self.WeaponFireSound`) _returnvalue_location (struct) 1.0 1.0 0.0 null null)
  (return))