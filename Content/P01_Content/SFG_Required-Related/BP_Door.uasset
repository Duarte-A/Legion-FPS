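; BP_Door is an interactable door that swings open and closed.
; OpenCloseDoor picks Open or Close from IsOpen and sets OpenCloseAnimation's play rate from OpenTime or CloseTime.
; Each event plays its own timeline to lerp the door's yaw between ClosedDoor and OpenedDoor.
; Close runs a separate Timeline that does not receive that play rate, and only Open's finish toggles IsOpen.
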(event `Event Open`
  (bind (_direction _door_rotation) (`Timeline|Open/ Close Animation`)
    (:`Update`
      (`SceneComponent.K2_SetRelativeRotation` (`self.Door`) (`KismetMathLibrary.MakeRotator` 0.0 0.0 (`KismetMathLibrary.Lerp` (`self.ClosedDoor`) (`self.OpenedDoor`) _door_rotation)) false false))
    (:`Finished`
      (set `self.IsOpen?` (not (`self.IsOpen?`))))))

(event `Event Close`
  (bind (_direction _door_rotation) (`Timeline|Timeline`)
    (:`Update`
      (`SceneComponent.K2_SetRelativeRotation` (`self.Door`) (`KismetMathLibrary.MakeRotator` 0.0 0.0 (`KismetMathLibrary.Lerp` (`self.OpenedDoor`) (`self.ClosedDoor`) _door_rotation)) false false))))

(fn `Open/Close Door`
  (params (Interactor :type "Character Object Reference"))
  (returns (`Did Interact?` :type Boolean))
  (bind _open__close_animation (`self.Open/ Close Animation`))
  (if (not (`self.IsOpen?`))
    (`TimelineComponent.SetPlayRate` _open__close_animation (/ 1.0 (`self.OpenTime`)))
    (`self.Event Open`)
    (else
      (`TimelineComponent.SetPlayRate` _open__close_animation (/ 1.0 (`self.CloseTime`)))
      (`self.Event Close`)))
  (return true))

(fn `UserConstructionScript`)