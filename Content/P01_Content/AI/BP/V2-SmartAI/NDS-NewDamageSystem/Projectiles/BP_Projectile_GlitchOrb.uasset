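; Glitch orb projectile for the AI damage system, built on a parent class that this Blueprint extends with spawn and lifetime handling.
; On BeginPlay it runs the parent logic, then sets whether its box collision ignores the instigator while moving, based on IgnoreInstigator.
; After a fixed delay it spawns an explosion particle effect at its location and destroys itself.
; It adds no overlap, tick or damage logic of its own.
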(event `self.ReceiveBeginPlay`
  (`parent.ReceiveBeginPlay`)
  (`PrimitiveComponent.IgnoreActorWhenMoving` (`self.BoxCollision`) (`self.GetInstigator`) (`self.IgnoreInstigator`))
  (`KismetSystemLibrary.Delay` 15.0)
  (`GameplayStatics.SpawnEmitterAtLocation` "/Game/FXVarietyPack/Particles/P_ky_explosion.P_ky_explosion" (`self.K2_GetActorLocation`))
  (`self.K2_DestroyActor`))

(fn `UserConstructionScript`
  (`parent.UserConstructionScript`))