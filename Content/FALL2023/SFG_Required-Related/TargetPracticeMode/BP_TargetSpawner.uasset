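; Target spawner that runs a timed aim-training round with music, score HUD and closing camera shake.
; StartSpawning, gated by DoOnce, spawns an initial batch, then a looping timer adds capped BP_Targets at random box points, oriented toward the camera.
; Targets receive a spawner reference, and UpdateMatchScore accumulates points on the HUD.
; When time expires, it destroys targets and updates the GameInstance session high and SaveGame all-time high if beaten.
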(event `UpdateMatchScore`
  (params (Points :type Integer))
  ;[0.005208 0.005208 0.005208] Update Match Score
  (bind _output_get (set `self.MatchScore` (+ Points (`self.MatchScore`))))
  (set `TextBlock.Text` (`KismetTextLibrary.Conv_IntToText` _output_get) (`/Game/FALL2023/SFG_Required-Related/TargetPracticeMode/WBP_Score.CurrentScore` (`self.WBP_Score`))))

(event `self.ReceiveBeginPlay`
  ;[0.08081 0.5188 1] BeginPlay
  (bind _returnvalue (`|CreateWidget` "/Game/FALL2023/SFG_Required-Related/TargetPracticeMode/WBP_Score.WBP_Score_C"))
  (`UserWidget.AddToViewport` _returnvalue 0)
  (set `self.WBP_Score` _returnvalue)
  (`|ExecutionSequence`
    (:`then_0`
      (bind _asgi_aim_trainer (cast `/Game/FirstPerson/Blueprints/GI_AimTrainer` (`GameplayStatics.GetGameInstance`)))
      (set `TextBlock.Text` (`KismetTextLibrary.Conv_IntToText` (`/Game/FirstPerson/Blueprints/GI_AimTrainer.Score` _asgi_aim_trainer)) (`/Game/FALL2023/SFG_Required-Related/TargetPracticeMode/WBP_Score.SessionHighScore` (`self.WBP_Score`))))
    (:`then_1`
      (bind _returnvalue_2 (`GameplayStatics.DoesSaveGameExist` "Score"))
      (if _returnvalue_2
        (bind _returnvalue_3 (`GameplayStatics.LoadGameFromSlot` "Score"))
        (bind _asbps_aim_trainer_save (cast `/Game/FALL2023/SFG_Required-Related/TargetPracticeMode/BPS_AimTrainer_Save` _returnvalue_3))
        (`TextBlock.SetText` (`/Game/FALL2023/SFG_Required-Related/TargetPracticeMode/WBP_Score.All-timeHigh` (`self.WBP_Score`)) (`KismetTextLibrary.Conv_IntToText` (`/Game/FALL2023/SFG_Required-Related/TargetPracticeMode/BPS_AimTrainer_Save.HighScore` _asbps_aim_trainer_save)))
        (else
          (bind _returnvalue_4 (`GameplayStatics.CreateSaveGameObject` "/Game/FALL2023/SFG_Required-Related/TargetPracticeMode/BPS_AimTrainer_Save.BPS_AimTrainer_Save_C"))
          (`GameplayStatics.SaveGameToSlot` _returnvalue_4 "Score"))))))

(event `StartSpawning`
  (bind _matchscore (`self.MatchScore`))
  (bind _matchscore_2 (`self.MatchScore`))
  ;[0.8021 0.6918 0] StartSpawning - Spawn a set amount of targets and start the loop of spawning targets
  (`/Engine/EditorBlueprintResources/StandardMacros.DoOnce` false
    (:`Completed`
      (bind _returnvalue (`GameplayStatics.SpawnSound2D` "/Game/FALL2023/SFG_Required-Related/TargetPracticeMode/Assets/Sounds/Music/WINGS-Intense-Action-Dramatic-Background-Music-_No-Copyright__Cue.WINGS-Intense-Action-Dramatic-Background-Music-_No-Copyright__Cue" 1.0 1.0 0.0 null))
      (set `self.AimTrainerMusic` _returnvalue)
      (`AudioComponent.FadeIn` _returnvalue 1.0 0.8 0.0 "Linear")
      (bind _returnvalue_2 (`KismetSystemLibrary.K2_SetTimerDelegate` (delegate `SpawnTarget`) 1.0 true))
      (set `self.TargetSpawner` _returnvalue_2)
      (for _ (range 9)
        (`self.SpawnTarget`))
      (`KismetSystemLibrary.Delay` 30.0)
      (`PlayerCameraManager.StartCameraShake` :`self` (`GameplayStatics.GetPlayerCameraManager` 0) :`ShakeClass` "/Game/Custom-Blueprints/ParkourComponent/CameraShakes/EndTraining.EndTraining_C")
      (`KismetSystemLibrary.K2_ClearAndInvalidateTimerHandle` (`self.TargetSpawner`))
      (bind _outactors (`GameplayStatics.GetAllActorsOfClass` "/Game/FALL2023/SFG_Required-Related/TargetPracticeMode/BP_Target.BP_Target_C"))
      (for _array_element _outactors
        (`self.K2_DestroyActor` _array_element))
      (`|ExecutionSequence`
        (:`then_0`
          (bind _asgi_aim_trainer (cast `/Game/FirstPerson/Blueprints/GI_AimTrainer` (`GameplayStatics.GetGameInstance`)))
          (if (> _matchscore_2 (`/Game/FirstPerson/Blueprints/GI_AimTrainer.Score` _asgi_aim_trainer))
            (bind _output_get (set `/Game/FirstPerson/Blueprints/GI_AimTrainer.Score` _matchscore_2 _asgi_aim_trainer))
            (set `TextBlock.Text` (`KismetTextLibrary.Conv_IntToText` _output_get) (`/Game/FALL2023/SFG_Required-Related/TargetPracticeMode/WBP_Score.SessionHighScore` (`self.WBP_Score`)))))
        (:`then_1`
          (bind _returnvalue_3 (`GameplayStatics.LoadGameFromSlot` "Score"))
          (bind _asbps_aim_trainer_save (cast `/Game/FALL2023/SFG_Required-Related/TargetPracticeMode/BPS_AimTrainer_Save` _returnvalue_3))
          (if (< (`/Game/FALL2023/SFG_Required-Related/TargetPracticeMode/BPS_AimTrainer_Save.HighScore` _asbps_aim_trainer_save) _matchscore)
            (`TextBlock.SetText` (`/Game/FALL2023/SFG_Required-Related/TargetPracticeMode/WBP_Score.All-timeHigh` (`self.WBP_Score`)) (`KismetTextLibrary.Conv_IntToText` _matchscore))
            (set `/Game/FALL2023/SFG_Required-Related/TargetPracticeMode/BPS_AimTrainer_Save.HighScore` _matchscore _asbps_aim_trainer_save)
            (`GameplayStatics.SaveGameToSlot` _asbps_aim_trainer_save "Score")))
        (:`then_2`
          (`AudioComponent.FadeOut` (`self.AimTrainerMusic`) 1.0 0.0 "Linear"))))))

(event `SpawnTarget`
  (bind _spawnarea (`self.SpawnArea`))
  ;[0.0169 0.1042 0] Spawn Targets
  (bind _outactors (`GameplayStatics.GetAllActorsOfClass` "/Game/FALL2023/SFG_Required-Related/TargetPracticeMode/BP_Target.BP_Target_C"))
  (if (<= (`KismetArrayLibrary.Array_Length` _outactors) 10)
    (bind _output_get (set `self.SpawnLocation` (`KismetMathLibrary.RandomPointInBoundingBox` (`SceneComponent.K2_GetComponentLocation` _spawnarea) (`BoxComponent.GetScaledBoxExtent` _spawnarea))))
    (bind (_returnvalue_roll _returnvalue_pitch _returnvalue_yaw) (`KismetMathLibrary.BreakRotator` (`KismetMathLibrary.FindLookAtRotation` _output_get (`SceneComponent.K2_GetComponentLocation` (`PlayerCameraManager.TransformComponent` (`GameplayStatics.GetPlayerCameraManager` 0))))))
    (`|SpawnActorFromClass` "/Game/FALL2023/SFG_Required-Related/TargetPracticeMode/BP_Target.BP_Target_C" (`KismetMathLibrary.MakeTransform` _output_get (`KismetMathLibrary.MakeRotator` _returnvalue_roll _returnvalue_pitch (- _returnvalue_yaw 90.0))) "AdjustIfPossibleButAlwaysSpawn" "MultiplyWithRoot" null self null)))

(fn `UserConstructionScript`
  (`BoxComponent.SetBoxExtent` (`self.SpawnArea`) (`self.BoxExtent`) true))