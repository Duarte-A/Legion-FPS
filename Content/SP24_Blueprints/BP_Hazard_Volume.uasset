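; BP_Hazard_Volume is a hazard area that deals periodic damage to actors inside its box trigger.
; Overlap events track actors that have a BPC_DamageSystem component, adding them on entry and removing them on exit.
; A looping timer started on BeginPlay sends each tracked actor a damage interface message at the DamageRate interval, using DamageAmount and a fixed damage type.
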(event `self.ReceiveBeginPlay`
  (`KismetSystemLibrary.K2_SetTimerDelegate` (delegate `Damage Tick`) (`self.Damage Rate`) true))

(event `Damage Tick`
  (for _array_element (`self.ActorsToDamage`)
    (message `/Game/P01_Content/AI/BP/V2-SmartAI/NDS-NewDamageSystem/Damage-Logic/BPI-NDS-Damagable.NDS-TakeDamage` _array_element (make `/Game/P01_Content/AI/BP/V2-SmartAI/NDS-NewDamageSystem/Damage-Logic/S_DamageInfo` (`self.Damage Amount`) "NewEnumerator4") self false)))

(event `self.Box Trigger.OnComponentBeginOverlap`
  (params (OverlappedComponent :type "PrimitiveComponent Object Reference") (OtherActor :type "Actor Object Reference") (OtherComp :type "PrimitiveComponent Object Reference") (OtherBodyIndex :type Integer) (bFromSweep :type Boolean) (SweepResult :type "HitResult Structure (by ref)"))
  (`/Engine/EditorBlueprintResources/StandardMacros.IsValid` (`self.GetComponentByClass` OtherActor "/Game/P01_Content/AI/BP/V2-SmartAI/NDS-NewDamageSystem/Damage-Logic/BPC_DamageSystem.BPC_DamageSystem_C")
    (:`Is Valid`
      (`KismetArrayLibrary.Array_Add` (`self.ActorsToDamage`) OtherActor))))

(event `self.Box Trigger.OnComponentEndOverlap`
  (params (OverlappedComponent :type "PrimitiveComponent Object Reference") (OtherActor :type "Actor Object Reference") (OtherComp :type "PrimitiveComponent Object Reference") (OtherBodyIndex :type Integer))
  (bind _returnvalue (`KismetArrayLibrary.Array_Find` (`self.ActorsToDamage`) OtherActor))
  (if (>= _returnvalue 0)
    (`KismetArrayLibrary.Array_Remove` (`self.ActorsToDamage`) _returnvalue)))

(fn `UserConstructionScript`)