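; BP_AmmoPickup is a collectible that refills reserve ammo for the weapon the player is holding.
; When the player character overlaps its CollectSphere, it casts to BP_FirstPersonCharacter and adds AmmoGain multiplied by the current weapon's magazine size to that weapon's reserve.
; It then plays a 2D sound, destroys itself and prints a message.
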(event `self.CollectSphere.OnComponentBeginOverlap`
  (params (OverlappedComponent :type "PrimitiveComponent Object Reference") (OtherActor :type "Actor Object Reference") (OtherComp :type "PrimitiveComponent Object Reference") (OtherBodyIndex :type Integer) (bFromSweep :type Boolean) (SweepResult :type "HitResult Structure (by ref)"))
  (bind _returnvalue (`GameplayStatics.GetPlayerCharacter` 0))
  (if (== OtherActor _returnvalue)
    (bind _asbp_first_person_character (cast `/Game/FirstPerson/Blueprints/Character/BP_FirstPersonCharacter` _returnvalue))
    (bind _currentweaponinhand (`/Game/FirstPerson/Blueprints/Character/BP_FirstPersonCharacter.CurrentWeaponInHand` _asbp_first_person_character))
    (set `/Game/WeaponSystemTesting/Blueprints/BP_WeaponBase.CurrentAmmoInReserve` (+ (`/Game/WeaponSystemTesting/Blueprints/BP_WeaponBase.CurrentAmmoInReserve` _currentweaponinhand) (* (`self.AmmoGain`) (`/Game/WeaponSystemTesting/Blueprints/BP_WeaponBase.MagSize` _currentweaponinhand))) _currentweaponinhand)
    (`GameplayStatics.PlaySound2D` "/Engine/VREditor/Sounds/VR_close_Cue.VR_close_Cue" 1.0 1.0 0.0 null null)
    (`self.K2_DestroyActor` self) ; Then destroy this projectile
    (`KismetSystemLibrary.PrintString` "More Bullets!")))

(fn `UserConstructionScript`)