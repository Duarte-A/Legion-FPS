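; Health pickup actor that heals the player when the player character hits it, and expires after 30 seconds if uncollected.
; On a collision hit from player 0, it plays a sound, heals a fraction of the player's max health set by ExtraHealth through NDS interface messages, then destroys itself.
; The damage, team and attack-token interface functions on the pickup itself are stubs returning default values.
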(event `self.ReceiveBeginPlay`
  ;[0 1 0] Life Span
  (`self.SetLifeSpan` 30.0))

(event `self.CollisionComponent.OnComponentHit`
  (params (HitComponent :type "PrimitiveComponent Object Reference") (OtherActor :type "Actor Object Reference") (OtherComp :type "PrimitiveComponent Object Reference") (NormalImpulse :type "Vector Structure") (Hit :type "HitResult Structure (by ref)"))
  ;[0 1 0] Pickup Collision
  (if (== OtherActor (`GameplayStatics.GetPlayerCharacter` 0))
    (`GameplayStatics.SpawnSoundAttached` "/Engine/VREditor/Sounds/VR_open_Cue.VR_open_Cue" HitComponent "None" (0.0 0.0 0.0) (struct) "KeepRelativeOffset" false 1.0 1.0 0.0 null null)
    (bind _maxhealth (message `/Game/P01_Content/AI/BP/V2-SmartAI/NDS-NewDamageSystem/Damage-Logic/BPI-NDS-Damagable.NDS-GetMaxHealth` OtherActor))
    (message `/Game/P01_Content/AI/BP/V2-SmartAI/NDS-NewDamageSystem/Damage-Logic/BPI-NDS-Damagable.NDS-Heal` OtherActor (* _maxhealth (`self.ExtraHealth`)))
    (`self.K2_DestroyActor` self) ; Then destroy this projectile
    (`KismetSystemLibrary.PrintString` "Health!")))

(fn `GetTeamNumber`
  (returns (TeamNumber :type Integer))
  (return 0))

(fn `NDS-GetCurrentHealth`
  (returns (Health :type "Float (double-precision)"))
  (return 0.0))

(fn `NDS-GetMaxHealth`
  (returns (MaxHealth :type "Float (double-precision)"))
  (return 0.0))

(fn `NDS-Heal`
  (params (Amount :type "Float (double-precision)" :default 0.0))
  (returns (NewHealth :type "Float (double-precision)"))
  (return 0.0))

(fn `NDS-IsAttacking`
  (returns (Attacking :type Boolean))
  (return false))

(fn `NDS-IsDead`
  (returns (Dead :type Boolean))
  (return false))

(fn `NDS-TakeDamage`
  (params (DamageInfo :type "/Game/P01_Content/AI/BP/V2-SmartAI/NDS-NewDamageSystem/Damage-Logic/S_DamageInfo Structure") (DamageCauser :type "Actor Object Reference") (wasHeadshot :type Boolean :default false))
  (returns (WasDamaged :type Boolean))
  (return false))

(fn `ReserveAttackToken`
  (params (Amount :type Integer :default 0))
  (returns (Success :type Boolean))
  (return false))

(fn `UserConstructionScript`)